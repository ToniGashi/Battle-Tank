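; Player-controlled tank Blueprint that handles driving, camera-rig aim and firing input.
; On BeginPlay it hands its turret, barrel and both track components to setter functions defined outside these graphs.
; Separate left and right throttle axes drive each track independently, and the fire action calls Fire.
; Frame-rate-independent aim axes yaw the Gimbal and pitch the SpringArm, without directly rotating turret or barrel here.
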(event `self.ReceiveBeginPlay`
  (`self.SetTurretReference` (`self.TankTurret1`))
  (`self.SetBarrelReference` (`self.TankBarrel`))
  (`self.SetTankTrackReference` (`self.Right Track`))
  (`self.SetTankTrackReference` (`self.Left Track`)))

(event `InputAxis|AimAzimuth`
  (params (AxisValue :type "Float (single-precision)"))
  ;[1 1 1] AimInputBinding
  (`SceneComponent.K2_AddLocalRotation` (`self.Gimbal`) (`KismetMathLibrary.MakeRotator` 0.0 0.0 (* AxisValue (`GameplayStatics.GetWorldDeltaSeconds`) 70.0)) false false))

(event `InputAxis|Left Throttle`
  (params (AxisValue :type "Float (single-precision)"))
  (`TankTrackMeshComponent.SetThrottle` (`self.Left Track`) AxisValue))

(event `InputAxis|Right Throttle`
  (params (AxisValue :type "Float (single-precision)"))
  (`TankTrackMeshComponent.SetThrottle` (`self.Right Track`) AxisValue))

(event `InputAxis|AimElevation`
  (params (AxisValue :type "Float (single-precision)"))
  ;[1 1 1] AimInputBinding
  (`SceneComponent.K2_AddLocalRotation` (`self.SpringArm`) (`KismetMathLibrary.MakeRotator` 0.0 (* AxisValue (`GameplayStatics.GetWorldDeltaSeconds`) 80.0)) false false))

(event `InputAction|Fire`
  (params (Key :type "Key Structure"))
  ;[1 1 1] AimInputBinding
  (:`Pressed`
    (`self.Fire`)))

(fn `UserConstructionScript`)